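; Actor that runs a voiced conversational agent, sending typed text from WB_TextInput to Dialogflow CX and animating the reply through Audio2Face.
; Chained HTTP requests extract the agent's response, synthesize it with Google TTS and write the decoded audio to a hardcoded Speech.wav path.
; Local Audio2Face REST calls then enable LiveLink streaming, generate emotion keys and play the track.
; Access token is refreshed manually; the JWT/OAuth generation is unfinished and unwired.
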(event Custom|CustomEvent
  (params (Input :type String))
  (bind _header (|MakeRequestHeader "Custom" "Content-type" "application/json"))
  (bind _output_get (Variables|Default|SetUserInput Input))
  (bind _output_get_2 (Variables|Default|SetUserText (Utilities|String|Append "{ \"queryInput\": { \"text\": { \"text\": \"" _output_get "\" }, \"languageCode\": \"en\" }, \"queryParams\": { \"timeZone\": \"Europe/London\" } }")))
  (bind _result_body (|HttpRequest (Variables|Default|GetAPIEndpoint) "Post" (|MakeRequestHeader "Custom" "Authorization" (Utilities|String|Append "Bearer " (Variables|Default|GetGCloudAccessToken)) "x-goog-user-project" "vcadialog" "Content-type" "application/json") _output_get_2)
    (:On%20Success
      (bind _outjsonobject (Class|JsonBlueprintFunctionLibrary|FromString _result_body))
      (bind _outvalue (|GetJsonField _outjsonobject "queryResult"))
      (bind _outvalue_2 (|GetJsonField _outvalue "responseMessages"))
      (bind _outvalue_3 (|GetJsonField (Utilities|Array|Get(acopy) _outvalue_2) "text"))
      (bind _outvalue_4 (|GetJsonField _outvalue_3 "text"))
      (bind _output_get_3 (Variables|Default|SetAgentResponse (Utilities|Array|Get(acopy) _outvalue_4)))
      (Development|PrintString _output_get_3 true true "(R=0.000000,G=0.660000,B=1.000000,A=1.000000)" 25.0)
      (bind _result_body_2 (|HttpRequest "https://texttospeech.googleapis.com/v1/text:synthesize?key=AIzaSyAisJJi89s7nAsCmQXaF0aksF9LSApHXn0" "Post" (|MakeRequestHeader "Custom" "Content-type" "application/json") (Utilities|String|Append "{ 
  \"input\": { 
    \"text\": \"" _output_get_3 (Variables|Default|GetPremiumTTS%28Chirp3%29)))
        (:On%20Success
          (bind _outjsonobject_2 (Class|JsonBlueprintFunctionLibrary|FromString _result_body_2))
          (bind _outvalue_5 (|GetJsonField _outjsonobject_2 "audioContent"))
          (Variables|Default|SetAudioB64 _outvalue_5)
          (Class|FileSDKBPLibrary|CreateDirectory "U:\\GitHub\\4th-Year-FYP\\VCA_FYP\\Speech\\" true)
          (Class|FileSDKBPLibrary|CreateFile "U:\\GitHub\\4th-Year-FYP\\VCA_FYP\\Speech\\Speech.wav" true false)
          (bind _output_get_4 (Variables|Default|SetAudioWAV (.Dest (Class|VaRestLibrary|Base64DecodeData (Variables|Default|GetAudioB64)))))
          (bind _returnvalue (Class|FileSDKBPLibrary|WriteBytestoFile "U:\\GitHub\\4th-Year-FYP\\VCA_FYP\\Speech\\Speech.wav" _output_get_4))
          (Development|PrintString ">>'Speech.wav' Updated" false _returnvalue "(R=0.032125,G=1.000000,B=0.000000,A=1.000000)" 1.0)
          (Class|HttpRequestProxyObject|CreateHttpRequestProxyObject "http://localhost:8011/A2F/Exporter/ActivateStreamLivelink" "POST" _header "{ 
  \"node_path\": \"/World/audio2face/StreamLivelink\", 
  \"value\": true 
}")
          (Class|HttpRequestProxyObject|CreateHttpRequestProxyObject "http://localhost:8011/A2F/Player/SetTrack" "POST" _header "{ 
  \"a2f_player\": \"/World/audio2face/Player\", 
  \"file_name\": \"Speech.wav\" 
}")
          (Class|HttpRequestProxyObject|CreateHttpRequestProxyObject "http://localhost:8011/A2F/A2E/GenerateKeys" "POST" _header "{ 
  \"a2f_instance\": \"/World/audio2face/CoreFullface\" 
}")
          (Class|HttpRequestProxyObject|CreateHttpRequestProxyObject "http://localhost:8011/A2F/Player/Play" "POST" _header "{ 
  \"a2f_player\": \"/World/audio2face/Player\" 
}"))))))

(event EventBeginPlay
  (bind _returnvalue (Game|GetPlayerController 0))
  (bind _returnvalue_2 (UserInterface|CreateWidget "/Game/WB_TextInput.WB_TextInput_C"))
  (UserInterface|Viewport|AddtoViewport _returnvalue_2 0)
  (EventDispatchers|BindEventtoOnUserTextUpdated _returnvalue_2 (delegate Custom|CustomEvent))
  (Input|SetInputModeGameandUI _returnvalue _returnvalue_2 "DoNotLock" true false)
  (Variables|/Script/Engine.PlayerController|SetbShowMouseCursor _returnvalue true))

(event Collision|EventActorBeginOverlap
  (params (OtherActor :type Actor%20Object%20Reference)))

(event Custom|Generate%20Token
  (bind _returnvalue (|EasyJwtSubsystem))
  (Class|EasyJwtSubsystem|InitGenerator _returnvalue (Variables|Default|GetPrivateKey) "HS256")
  (bind _returnvalue_2 (Class|EasyJwtSubsystem|GetClaims _returnvalue (Variables|Default|GetTokenURI)))
  (bind _returnvalue_3 (Class|EasyJwtSubsystem|GenerateJwtToken _returnvalue false _returnvalue_2 _returnvalue_2 0 3300))
  (Variables|Default|SetAccToken _returnvalue_3))

(fn ConstructionScript
  (Variables|Default|SetAPIEndpoint (Utilities|String|Append "https://dialogflow.googleapis.com/v3/projects/" (Variables|Default|GetProjectID) "/locations/" (Variables|Default|GetLocation) "/agents/" (Variables|Default|GetAgentID) "/sessions/" (Variables|Default|GetSessionID) ":detectIntent")))

(fn OAuthTokenAuto-Generator
  (bind _outjsonobject (Class|JsonBlueprintFunctionLibrary|FromFile (Utilities|Struct|MakeFilePath "\"U:\\GitHub\\API Keys(Not the best idea to store them on Github)\\DialogFlow\\vcadialog-5db11e53cb62.json\"")))
  (bind _outvalue (|GetJsonField _outjsonobject "client_email"))
  (Variables|Default|SetClientEmail _outvalue)
  (bind _outvalue_2 (|GetJsonField _outjsonobject "private_key"))
  (Variables|Default|SetPrivateKey _outvalue_2)
  (bind _outvalue_3 (|GetJsonField _outjsonobject "token_uri"))
  (bind _output_get (Variables|Default|SetTokenURI _outvalue_3))
  (Class|HttpRequestProxyObject|CreateHttpRequestProxyObject _output_get "POST" (|MakeRequestHeader "Custom" "Content-type" "application/json") (Utilities|String|Append "{ \"grant_type\": \"urn:ietf:params:oauth:grant-type:jwt-bearer\", \"assertation\": \"" "" "\" }")))